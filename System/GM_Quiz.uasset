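; GM_Quiz is the game mode for a joke quiz, sending each player a multiple-choice question about punchlines.
; After the first login and a short delay, a temporary hook begins the dad joke category once.
; BeginCategory shuffles that category's joke pool, then AskQuestion records the correct punchline for the current index, shuffles the choices and passes both joke and choices to every PC_Quiz controller in the PlayerArray.
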(event `self.K2_PostLogin`
  (params (NewPlayer :type "PlayerController Object Reference"))
  (`KismetSystemLibrary.Delay` 2.0)
  ; Temp
  (`/Engine/EditorBlueprintResources/StandardMacros.DoOnce` false
    (:`Completed`
      (`self.BeginCategory#` "/Game/Jokes/Dad_Jokes/CAT_Dadjoke.CAT_Dadjoke"))))

(event `BeginCategory#`
  (params (Category :type "/Game/Jokes/DA_category Object Reference"))
  (bind _output_get (set `self.CurrentCategory` Category))
  (bind _output_get_2 (set `self.Current Joke Pool` (`/Game/Jokes/DA_category.JokePool` _output_get)))
  (`KismetArrayLibrary.Array_Shuffle` _output_get_2)
  (`self.AskQuestion`))

(event `AskQuestion`
  (bind _output (`|GetArrayItem` (`self.Current Joke Pool`) (`self.CurrentQuestionIndex`)))
  (bind _punchlines (`/Game/Jokes/DA_Joke.PunchLines` _output))
  (set `self.Correct Answer` (`|GetArrayItem` _punchlines (`/Game/Jokes/DA_Joke.CorrectAnswer` _output)))
  (bind _output_get (set `self.Punch Lines` _punchlines))
  (`KismetArrayLibrary.Array_Shuffle` _output_get)
  (for _array_element (`GameStateBase.PlayerArray` (`GameplayStatics.GetGameState`))
    (bind _aspc_quiz (cast `/Game/System/PC_Quiz` (`PlayerState.GetPlayerController` _array_element)))
    (`/Game/System/PC_Quiz.AskQuestion` _aspc_quiz (`|GetArrayItem` (`self.Current Joke Pool`) (`self.CurrentQuestionIndex`)) (`self.Punch Lines`))))

(fn `UserConstructionScript`)