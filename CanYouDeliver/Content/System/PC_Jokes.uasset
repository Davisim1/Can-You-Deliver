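; Player controller for a joke-and-punchline quiz game, using UI-only input and bridging the HUD and game state.
; AskJoke starts a 10-second question timer and sends the joke and punchlines to the HUD.
; SetAnswer forwards the locked-in answer and remaining time to the game state.
; TimerExpired scans every player's timer and, as wired, triggers the answer reveal when one is still active, not when all have finished.
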(event `self.ReceiveBeginPlay`
  (`WidgetBlueprintLibrary.SetInputMode_UIOnlyEx` self null))

(event `AskJoke`
  (params (Joke :type "/Game/Jokes/DA_Joke Object Reference") (`Punch lines` :type "Array of Text"))
  (`KismetSystemLibrary.PrintString` "Hello")
  (`self.Start Timer`)
  (bind _ashud_jokes (cast `/Game/System/HUD_Jokes` (`self.GetHUD`)))
  (`/Game/System/HUD_Jokes.AskJoke` _ashud_jokes Joke `Punch lines`))

(event `Client_RevealAnswers`
  (bind _ashud_jokes (cast `/Game/System/HUD_Jokes` (`self.GetHUD` (`GameplayStatics.GetPlayerController` 0))))
  (`/Game/System/HUD_Jokes.RevealAnswers` _ashud_jokes))

(event `SetAnswer`
  (params (Answer :type Text) (TimeRemaining :type "Float (double-precision)"))
  (bind _asgs_jokes (cast `/Game/System/GS_Jokes` (`GameplayStatics.GetGameState`)))
  (`/Game/System/GS_Jokes.MC_UpdateLockedInAnswer` _asgs_jokes (`self.PlayerState`) Answer TimeRemaining))

(event `TimerExpired`
  (bind _return (`self.CheckTimerStatus`))
  (if (not _return)
    (`self.Client_RevealAnswers`)))

(fn `CheckTimerStatus`
  (returns (Return :type Boolean))
  (for _array_element (`GameStateBase.PlayerArray` (`GameplayStatics.GetGameState`))
    (bind _aspc_jokes (cast `/Game/System/PC_Jokes` (`PlayerState.GetPlayerController` _array_element)))
    (if (`KismetSystemLibrary.K2_IsTimerActiveHandle` (`/Game/System/PC_Jokes.QuestionTimer` _aspc_jokes))
      (return false)))
  (return true))

(fn `Start Timer`
  (bind _returnvalue (`KismetSystemLibrary.K2_SetTimerDelegate` (`|CreateDelegate` :!event `TimerExpired`) 10.0))
  (set `self.QuestionTimer` _returnvalue))

(fn `UserConstructionScript`)